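; Base actor for a static mesh object that can be selected and edited through its BPC_DragTransformActor component.
; The component's init data supplies a mesh name, which is resolved under FilePath via an Asset Registry object-path lookup and applied to the mesh.
; Clicking the mesh calls OnlyShowSelfEditor on the component, and selection changes toggle custom depth rendering on the mesh.
; GetEditorComponent exposes the component to other Blueprints.
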(event OnInitDataChange(BPC_DragTransformActor)
  (params (Data :type String))
  (Components|StaticMesh|SetStaticMesh (Variables|Default|GetStaticMesh) (CallFunction|FindStaticMeshbyName (Variables|Default|GetFile%20Path) Data)))

(event OnClicked(StaticMesh)
  (params (TouchedComponent :type Primitive%20Component%20Object%20Reference) (ButtonPressed :type Key%20Structure :default "None"))
  (Default|OnlyShowSelfEditor (Variables|Default|GetBPC_DragTransformActor) false))

(event OnSelectStateChange(BPC_DragTransformActor)
  (params (Select :type Boolean))
  (Rendering|SetRenderCustomDepth (Variables|Default|GetStaticMesh) Select))

(event EventBeginPlay)

(event Collision|EventActorBeginOverlap
  (params (OtherActor :type Actor%20Object%20Reference)))

(event EventTick
  (params (DeltaSeconds :type Float%20%28single-precision%29)))

(fn ConstructionScript)

(fn FindStaticMeshbyName
  (params (FilePath :type String) (MeshName :type String))
  (bind _returnvalue (Utilities|String|Append FilePath MeshName "." MeshName))
  (bind _returnvalue_2 (Utilities|String|StringToName _returnvalue))
  (bind _returnvalue_3 (Class|AssetRegistry|GetAssetbyObjectPath (Class|AssetRegistryHelpers|GetAssetRegistry) _returnvalue_2 false))
  (Development|PrintString (Utilities|String|ToString(Name) _returnvalue_2) false true "(R=0.000000,G=0.000000,B=0.000000,A=1.000000)" 1e+01)
  (bind _asstatic_mesh (Utilities|Casting|CastToStaticMesh (Class|AssetRegistryHelpers|GetAsset _returnvalue_3)))
  (return _asstatic_mesh))

(fn GetEditorComponent
  (return (Variables|Default|GetBPC_DragTransformActor)))