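; BP_DragCharacter_Base is a base character that can be selected by clicking and moved through its AI controller.
; Clicking the mesh calls OnlyShowSelfEditor on its BPC_DragTransformActor component, whose selection changes toggle custom depth on the mesh.
; MovetoTarget sends the character to a navmesh-projected location only while it is selected.
; GetEditorComponent exposes the drag transform component to callers.
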(event OnSelectStateChange(BPC_DragTransformActor)
  (params (Select :type Boolean))
  (Rendering|SetRenderCustomDepth (Variables|Character|GetMesh) Select))

(event OnClicked(Mesh)
  (params (TouchedComponent :type Primitive%20Component%20Object%20Reference) (ButtonPressed :type Key%20Structure))
  (Default|OnlyShowSelfEditor (Variables|Default|GetBPC_DragTransformActor) false))

(event EventBeginPlay)

(event Collision|EventActorBeginOverlap
  (params (OtherActor :type Actor%20Object%20Reference)))

(event EventTick
  (params (DeltaSeconds :type Float%20%28single-precision%29)))

(event EventMovetoTarget
  (params (TargetLocation :type Vector :default "0, 0, 0"))
  (if (Variables|/TransformGizmoDepot/TransformGizmo/BPC_DragTransformActor.BPC_DragTransformActor_C|GetSelectState (Variables|Default|GetBPC_DragTransformActor))
    (AI|Navigation|MovetoLocation (AI|GetAIController self) TargetLocation 1e+01 true true true true 0)))

(fn ConstructionScript)

(fn GetEditorComponent
  (return (Variables|Default|GetBPC_DragTransformActor)))