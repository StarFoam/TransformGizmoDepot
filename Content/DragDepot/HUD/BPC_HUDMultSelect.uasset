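; BPC_HUDMultSelect is a HUD component that provides drag-box multi-selection of editor actors.
; Start, update and stop functions track the mouse drag corners, while a DrawOpen flag enables or disables the feature.
; While dragging, RunDrawSelectBox draws an outlined, filled box using SelectBoxStyle and rebuilds the selection through GetActorsInSelectionRectangle.
; Each pass clears prior highlights, then calls SetSelectActor on actors that have a BPCDragEditorActor component.
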(fn ClearSelectActor
  (for _array_element (Variables|Private|GetSelectedActorList)
    (Utilities|IsValid _array_element
      (:Is%20Valid
        (if (.bSuccess (CallFunction|GetEditorComponentActor _array_element))
          (Default|SetSelectActor (.AsBPC%20Drag%20Editor%20Actor (CallFunction|GetEditorComponentActor _array_element)) false)))))
  (Utilities|Array|Clear (Variables|Private|GetSelectedActorList))
  (return))

(fn DrawSelect2DBox
  (params (StartPosition :type Vector%202D%20Structure) (EndPosition :type Vector%202D%20Structure) (LineColor :type Linear%20Color%20Structure :default "(R=0.099899,G=0.603828,B=0.401978,A=0.498039)") (LineThickness :type Float%20%28single-precision%29) (RectColor :type Linear%20Color%20Structure :default "(R=0.135633,G=0.630757,B=0.450786,A=0.196078)"))
  (bind (_x _y) (Math|Vector2D|BreakVector2D StartPosition))
  (bind (_x_2 _y_2) (Math|Vector2D|BreakVector2D EndPosition))
  (bind _returnvalue (Game|GetPlayerController 0))
  (bind _downposition (Variables|Private|GetDownPosition))
  (bind _releaseposition (Variables|Private|GetReleasePosition))
  (bind _returnvalue_2 (HUD|GetHUD _returnvalue))
  (bind (_x_3 _y_3) (Math|Vector2D|BreakVector2D _releaseposition))
  (bind (_x_4 _y_4) (Math|Vector2D|BreakVector2D _downposition))
  (Utilities|FlowControl|Sequence
    (:then_0
      (Class|HUD|DrawLine _returnvalue_2 _x _y _x_2 _y LineColor LineThickness) ; top
    )
    (:then_1
      (Class|HUD|DrawLine _returnvalue_2 _x _y_2 _x_2 _y_2 LineColor LineThickness) ; bottom
    )
    (:then_2
      (Class|HUD|DrawLine _returnvalue_2 _x_2 _y _x_2 _y_2 LineColor LineThickness) ; right
    )
    (:then_3
      (Class|HUD|DrawLine _returnvalue_2 _x _y _x _y_2 LineColor LineThickness) ; Left
    )
    (:then_4
      (HUD|DrawRect _returnvalue_2 RectColor _x_4 _y_4 (- _x_3 _x_4) (- _y_3 _y_4)))
    (:then_5
      (return))))

(fn UpdateReleasePosition
  (bind _returnvalue (Game|GetPlayerController 0))
  (bind (_locationx _locationy) (Game|Player|GetMousePosition _returnvalue))
  (Variables|Private|SetReleasePosition (Math|Vector2D|MakeVector2D _locationx _locationy)))

(fn RunDrawSelectBox
  (bind _selectboxstyle (Variables|Default|GetSelectBoxStyle))
  (bind (_linecolor _linethickness _rectcolor) (Utilities|Struct|BreakS_SelectBoxStyle _selectboxstyle))
  (if (Variables|Private|GetDrawOpen)
    (if (Variables|Private|GetIsDrawingRect)
      (Private|DrawSelect2DBox (Variables|Private|GetDownPosition) (Variables|Private|GetReleasePosition) _linecolor _linethickness _rectcolor)
      (CallFunction|ClearSelectActor)
      (Variables|Private|SetSelectedActorList (Class|HUD|GetActorsinSelectionRectangle (HUD|GetHUD (Game|GetPlayerController 0)) "/Script/Engine.Actor" (Variables|Private|GetDownPosition) (Variables|Private|GetReleasePosition) false false))
      (for _array_element (Variables|Private|GetSelectedActorList)
        (if (.bSuccess (CallFunction|GetEditorComponentActor _array_element))
          (Default|SetSelectActor (.AsBPC%20Drag%20Editor%20Actor (CallFunction|GetEditorComponentActor _array_element)) true))))))

(fn StartDrawHUD
  (bind _returnvalue (Game|GetPlayerController 0))
  (bind (_locationx _locationy) (Game|Player|GetMousePosition _returnvalue))
  (bind _returnvalue_2 (Math|Vector2D|MakeVector2D _locationx _locationy))
  (Variables|Private|SetIsDrawingRect true)
  (Variables|Private|SetDownPosition _returnvalue_2)
  (Variables|Private|SetReleasePosition _returnvalue_2))

(fn StopDrawHUD
  (Variables|Private|SetIsDrawingRect false))

(fn UpdateDrawState
  (params (DrawState :type Boolean))
  (Variables|Private|SetDrawOpen DrawState))