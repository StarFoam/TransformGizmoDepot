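; Manager actor that persists drag-depot editor actors across sessions, gated by open and save/load flags.
; On BeginPlay it loads or creates a BP_DragSave from the GameDragData slot, respawns each saved class and transform, then initializes its drag-editor component with the stored data.
; On EndPlay it gathers actors implementing BPI_TransformComponent, collects data from editor components that need saving, and writes the slot asynchronously.
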(event Custom|Load%20Drag%20Actor
  (if (Variables|Default|GetDragDepotOpen)
    (if (Variables|Default|GetDepotSaveLoad)
      (bind _returnvalue (SaveGame|LoadGamefromSlot "GameDragData"))
      (bind _asbp_drag_save (Utilities|Casting|CastToBP_DragSave _returnvalue)
        (:then
          (Variables|Default|SetAs%20BP%20Drag%20Actor%20Save _asbp_drag_save))
        (:CastFailed
          (bind _returnvalue_2 (SaveGame|CreateSaveGameObject "/TransformGizmoDepot/DragDepot/Blueprint/BP_DragSave.BP_DragSave_C"))
          (Variables|Default|SetAs%20BP%20Drag%20Actor%20Save _returnvalue_2)))
      (if (Utilities|Array|IsValidIndex (Variables|/TransformGizmoDepot/DragDepot/Blueprint/BP_DragSave.BP_DragSave_C|GetEditorSaveData (Variables|Default|GetAs%20BP%20Drag%20Actor%20Save)))
        (for _array_element (Variables|/TransformGizmoDepot/DragDepot/Blueprint/BP_DragSave.BP_DragSave_C|GetEditorSaveData (Variables|Default|GetAs%20BP%20Drag%20Actor%20Save))
          (bind _returnvalue_3 (Game|SpawnActorfromClass (.Class (Utilities|Struct|BreakS_DragSaveData _array_element)) (.Transform (Utilities|Struct|BreakS_DragSaveData _array_element)) "AlwaysSpawn" 0 0))
          (Default|InitializeData (.AsBPC%20Drag%20Editor%20Actor (CallFunction|GetEditorComponentActor _returnvalue_3)) (.Data (Utilities|Struct|BreakS_DragSaveData _array_element))))))))

(event Custom|SaveDragActor
  (bind _as_bp_drag_actor_save (Variables|Default|GetAs%20BP%20Drag%20Actor%20Save))
  (if (Variables|Default|GetDragDepotOpen)
    (if (Variables|Default|GetDepotSaveLoad)
      (Utilities|IsValid (Variables|Default|GetAs%20BP%20Drag%20Actor%20Save)
        (:Is%20Valid
          (bind _outactors (Actor|GetAllActorswithInterface "/TransformGizmoDepot/TransformGizmo/Blueprint/BPI_TransformComponent.BPI_TransformComponent_C"))
          (for _array_element _outactors
            (if (.bSuccess (CallFunction|GetEditorComponentActor _array_element))
              (bind (_needtosave _savedata) (Default|SavetoLevelData (.AsBPC%20Drag%20Editor%20Actor (CallFunction|GetEditorComponentActor _array_element))))
              (if _needtosave
                (Utilities|Array|Add (Variables|Default|GetEditor%20Save%20Data) _savedata))))
          (Variables|/TransformGizmoDepot/DragDepot/Blueprint/BP_DragSave.BP_DragSave_C|SetEditorSaveData _as_bp_drag_actor_save (Variables|Default|GetEditor%20Save%20Data))
          (|AsyncSaveGametoSlot _as_bp_drag_actor_save "GameDragData"))))))

(event EventBeginPlay
  (CallFunction|LoadDragActor))

(event EventTick
  (params (DeltaSeconds :type Float%20%28single-precision%29)))

(event EventEndPlay
  (params (EndPlayReason :type EEndPlayReason%20Enum :default "Destroyed"))
  (CallFunction|SaveDragActor))

(fn ConstructionScript)