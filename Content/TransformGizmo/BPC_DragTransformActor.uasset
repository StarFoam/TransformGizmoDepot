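; Actor component that makes its owner selectable and editable with a runtime transform gizmo.
; Showing the gizmo spawns BP_TransformGizmo with editor settings, disables owner collision and marks it selected, optionally gated by the drag controller's mode.
; Transform edits update the owner, notify BPI_DragTransformUI widgets and sync the gizmo when made externally.
; It also handles exclusive gizmo display, guarded deletion and save data of class, custom data and transform.
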(event EventBeginPlay)

(event EventTick
  (params (DeltaSeconds :type Float%20%28single-precision%29)))

(fn SetSelectActor
  (params (IsSelect :type Boolean))
  (bind _output_get (Variables|Run|SetSelectState IsSelect))
  (Default|CallOnSelectStateChange _output_get))

(fn ShowTransformGizmo
  (params (Show :type Boolean))
  (bind _editorgizmosetting (Variables|Default|GetEditorGizmoSetting))
  (bind (_arrowvisible _rotateactive _editorgizmoscale _editormode _coordinatesystem _locationgridsnap _rotationgridsnap _scalegridsnap _valuewidgetvisible _cameravisible) (Utilities|Struct|BreakS_CompleteTransformGizmoSetting _editorgizmosetting))
  (if Show
    (bind _returnvalue (Game|SpawnActorfromClass "/TransformGizmoDepot/TransformGizmo/BP_TransformGizmo.BP_TransformGizmo_C" (Math|Transform|MakeTransform "0, 0, 0" "0, 0, 0" "1,1,1") "AlwaysSpawn" (Components|GetOwner) (Transformation|GetActorTransform (Components|GetOwner)) _arrowvisible _rotateactive _editorgizmoscale _editormode _coordinatesystem _locationgridsnap _rotationgridsnap _scalegridsnap _valuewidgetvisible _cameravisible 0))
    (Variables|Default|SetEditor _returnvalue)
    (Collision|SetActorEnableCollision (Components|GetOwner) false)
    (CallFunction|SetSelectActor true)
    (bind _foundwidgets (Class|WidgetBlueprintLibrary|GetAllWidgetswithInterface "/TransformGizmoDepot/DragDepot/Blueprint/BPI_DragTransformUI.BPI_DragTransformUI_C" false))
    (Class|BPIDragTransformUI|SetSelectActorTransform(Message) _foundwidgets (Components|GetOwner) (Transformation|GetActorTransform (Components|GetOwner)) true)
    (else
      (Utilities|IsValid (Variables|Default|GetEditor)
        (:Is%20Valid
          (Actor|DestroyActor (Variables|Default|GetEditor))
          (Collision|SetActorEnableCollision (Components|GetOwner) true)
          (CallFunction|SetSelectActor false))))))

(fn DestroyEditorActor
  (bind _editor (Variables|Default|GetEditor))
  (if (Variables|Default|GetCanDestroyByInterface)
    (Default|CallOnActorDestory)
    (Actor|DestroyActor (Components|GetOwner))
    (Utilities|IsValid _editor
      (:Is%20Valid
        (Actor|DestroyActor _editor)))))

(fn EditTransformEditorActor
  (params (Transform :type Transform) (FromEditor :type Boolean))
  (bind _editor (Variables|Default|GetEditor))
  (Default|CallOnTransformEditorChange Transform FromEditor)
  (Transformation|SetActorTransform (Components|GetOwner) Transform)
  (bind _foundwidgets (Class|WidgetBlueprintLibrary|GetAllWidgetswithInterface "/TransformGizmoDepot/DragDepot/Blueprint/BPI_DragTransformUI.BPI_DragTransformUI_C" false))
  (Class|BPIDragTransformUI|SetSelectActorTransform(Message) _foundwidgets (Components|GetOwner) (Transformation|GetActorTransform (Components|GetOwner)) false)
  (if (not FromEditor)
    (Utilities|IsValid _editor
      (:Is%20Valid
        (Default|UpdateTransform _editor Transform)))))

(fn InitializeData
  (params (Data :type String))
  (bind _output_get (Variables|Run|SetData Data))
  (Default|CallOnInitDataChange _output_get))

(fn SavetoLevelData
  (bind _returnvalue (Components|GetOwner))
  (return (Variables|Default|GetNeedToSave) (Utilities|Struct|MakeS_DragSaveData (Utilities|GetClass _returnvalue) (Variables|Run|GetData) (Transformation|GetActorTransform _returnvalue))))

(fn OnlyShowSelfEditor
  (params (Condition :type Boolean))
  (bind _actorcomponentlist (CallFunction|GetEditorComponentActorList))
  (for _array_element _actorcomponentlist
    (CallFunction|ShowTransformGizmo _array_element false))
  (if (Variables|Default|GetNeedEditorModeToShowGizmo)
    (if (Utilities|Enum|Equal(Enum) (Variables|/TransformGizmoDepot/TransformGizmo/BPC_DragTransformController.BPC_DragTransformController_C|GetDragMode (.AsBPC%20Drag%20Controller (CallFunction|GetEditorComponentController))) "NewEnumerator1")
      (CallFunction|ShowTransformGizmo true))
    (else
      (CallFunction|ShowTransformGizmo true))))