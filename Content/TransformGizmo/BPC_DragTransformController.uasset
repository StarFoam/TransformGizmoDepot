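; Player-side component that controls runtime editing of placed actors: drag placement, gizmo interaction, selection and deletion.
; Tick snaps the dragged actor, collision disabled, to the cursor hit and reports its transform to UI, while a cursor trace drives gizmo hover.
; Draw-button functions forward gizmo clicks and toggle HUD box drawing.
; Cyclable Normal, Editor and MultipleChoice modes reset selection or gizmos; MultipleChoice also sends move orders to characters.
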(event EventBeginPlay
  (bind _returnvalue (UserInterface|CreateWidget "/TransformGizmoDepot/TransformGizmo/UI/WBP_TranslucentMouse.WBP_TranslucentMouse_C"))
  (bind _output_get (Variables|Default|SetUI_TranslucentMouse _returnvalue))
  (Class|PlayerController|SetMouseCursorWidget (Game|GetPlayerController 0) "SlashedCircle" _output_get))

(event EventTick
  (params (DeltaSeconds :type Float%20%28single-precision%29))
  (bind _returnvalue (Game|GetPlayerController 0))
  (bind _dragactor (Variables|Default|GetDragActor))
  (bind _dragactor_2 (Variables|Default|GetDragActor))
  (bind _dragactor_3 (Variables|Default|GetDragActor))
  (bind (_hitresult _returnvalue_2) (Game|Player|GetHitResultUnderCursorbyChannel _returnvalue "TraceTypeQuery3" true))
  (bind (_asbpc_drag_editor_actor _bsuccess) (CallFunction|GetEditorComponentActor _dragactor_2))
  (bind (_returnvalue_3 _location _rotation) (CallFunction|GetMouseHitLocationandRotation _dragactor_3))
  (bind (_bblockinghit _binitialoverlap _time _distance _location_2 _impactpoint _normal _impactnormal _physmat _hitactor _hitcomponent) (Collision|BreakHitResult _hitresult))
  (bind _usedefaultrotate (Variables|/TransformGizmoDepot/TransformGizmo/BPC_DragTransformActor.BPC_DragTransformActor_C|GetUseDefaultRotate _asbpc_drag_editor_actor))
  (bind _returnvalue_4 (Math|Rotator|SelectRotator "0, 0, 0" _rotation _usedefaultrotate))
  (Utilities|FlowControl|Sequence
    (:then_0
      (if (Variables|Default|GetIsDraging)
        (Utilities|IsValid (Variables|Default|GetDragActor)
          (:Is%20Valid
            (if _returnvalue_3
              (if _bsuccess
                (Transformation|SetActorLocationAndRotation _dragactor_2 _location _returnvalue_4)
                (bind _foundwidgets (Class|WidgetBlueprintLibrary|GetAllWidgetswithInterface "/TransformGizmoDepot/DragDepot/Blueprint/BPI_DragTransformUI.BPI_DragTransformUI_C" false))
                (Class|BPIDragTransformUI|SetSelectActorTransform(Message) _foundwidgets _dragactor (Math|Transform|MakeTransform _location _returnvalue_4 (Transformation|GetActorScale3D _dragactor)) false)))))))
    (:then_1
      (if _returnvalue_2
        (Class|BPITransformGizmo|HoverComponent(Message) _hitactor _hitcomponent)
        (else
          (bind _outactors (Actor|GetAllActorswithInterface "/TransformGizmoDepot/TransformGizmo/Blueprint/BPI_Transform_Gizmo.BPI_Transform_Gizmo_C"))
          (Class|BPITransformGizmo|UnHoverComponent(Message) _outactors))))))

(fn DrawButtonDown
  (bind _returnvalue (Game|GetPlayerController 0))
  (bind _hitresult (Game|Player|GetHitResultUnderCursorbyChannel _returnvalue "TraceTypeQuery3" true))
  (bind (_bblockinghit _binitialoverlap _time _distance _location _impactpoint _normal _impactnormal _physmat _hitactor _hitcomponent) (Collision|BreakHitResult _hitresult))
  (Variables|Default|SetIsDrawButtonDown true)
  (Default|StartDrawHUD (.AsBPC%20Drag%20Editor%20HUD (CallFunction|GetEditorComponentHUD)))
  (Input|SetInputModeGameandUI (Game|GetPlayerController 0) 0 "DoNotLock" true)
  (Class|BPITransformGizmo|ClickComponent(Message) _hitactor _hitcomponent)
  (return (Variables|Default|GetDragMode)))

(fn DrawButtonRelease
  (Variables|Default|SetIsDrawButtonDown false)
  (Default|StopDrawHUD (.AsBPC%20Drag%20Editor%20HUD (CallFunction|GetEditorComponentHUD)))
  (Input|SetInputModeGameandUI (Game|GetPlayerController 0) 0 "LockOnCapture" true)
  (CallFunction|UpdateDragActor false)
  (bind _outactors (Actor|GetAllActorswithInterface "/TransformGizmoDepot/TransformGizmo/Blueprint/BPI_Transform_Gizmo.BPI_Transform_Gizmo_C"))
  (Class|BPITransformGizmo|ReleaseDragButton(Message) _outactors)
  (return (Variables|Default|GetDragMode)))

(fn DestroySelectActor
  (bind _outactors (Actor|GetAllActorsOfClass "/TransformGizmoDepot/TransformGizmo/BP_TransformGizmo.BP_TransformGizmo_C"))
  (for _array_element _outactors
    (Default|DestroyEditorActor (.AsBPC%20Drag%20Editor%20Actor (CallFunction|GetEditorComponentActor (Components|GetOwner _array_element)))))
  (bind _foundwidgets (Class|WidgetBlueprintLibrary|GetAllWidgetswithInterface "/TransformGizmoDepot/DragDepot/Blueprint/BPI_DragTransformUI.BPI_DragTransformUI_C" false))
  (Class|BPIDragTransformUI|HiddenTransformPanel(Message) _foundwidgets)
  (bind _actorcomponentlist (CallFunction|GetEditorComponentActorList))
  (for _array_element_2 _actorcomponentlist
    (if (Variables|/TransformGizmoDepot/TransformGizmo/BPC_DragTransformActor.BPC_DragTransformActor_C|GetSelectState _array_element_2)
      (Default|DestroyEditorActor _array_element_2))))

(fn UpdateDragActor
  (params (Open :type Boolean) (Actor :type Actor%20Object%20Reference))
  (bind _output_get (Variables|Default|SetIsDraging Open))
  (if _output_get
    (bind _output_get_2 (Variables|Default|SetDragActor Actor))
    (Collision|SetActorEnableCollision _output_get_2 false)
    (else
      (Utilities|IsValid (Variables|Default|GetDragActor)
        (:Is%20Valid
          (Collision|SetActorEnableCollision (Variables|Default|GetDragActor) true)
          (Variables|Default|SetDragActor 0))))))

(fn MoveSelectPawnto
  (if (Utilities|Enum|Equal(Enum) (Variables|Default|GetDragMode) "NewEnumerator2")
    (bind _outactors (Actor|GetAllActorswithInterface "/TransformGizmoDepot/DragDepot/Blueprint/BPI_Character.BPI_Character_C"))
    (Class|BPICharacter|MovetoTarget(Message) _outactors (.Location (CallFunction|GetMouseHitLocationandRotation)))))

(fn UpdateDragMode
  (params (Mode :type E_DragMode%20Enum :default "NewEnumerator0"))
  (bind (_asbpc_drag_editor_hud _bsuccess) (CallFunction|GetEditorComponentHUD))
  (Variables|Default|SetDragMode Mode)
  (bind _foundwidgets (Class|WidgetBlueprintLibrary|GetAllWidgetswithInterface "/TransformGizmoDepot/DragDepot/Blueprint/BPI_DragTransformUI.BPI_DragTransformUI_C" false))
  (Class|BPIDragTransformUI|ChangeDragMode(Message) _foundwidgets (Variables|Default|GetDragMode))
  (if _bsuccess
    (Default|UpdateDrawState _asbpc_drag_editor_hud (Utilities|Enum|Equal(Enum) (Variables|Default|GetDragMode) "NewEnumerator2")))
  (bind _foundwidgets_2 (Class|WidgetBlueprintLibrary|GetAllWidgetswithInterface "/TransformGizmoDepot/DragDepot/Blueprint/BPI_DragTransformUI.BPI_DragTransformUI_C" false))
  (Class|BPIDragTransformUI|ChangeDragMode(Message) _foundwidgets_2 (Variables|Default|GetDragMode))
  (switch Utilities|FlowControl|Switch|SwitchonE_DragMode (Variables|Default|GetDragMode)
    (:NewEnumerator0
      (bind _actorcomponentlist (CallFunction|GetEditorComponentActorList))
      (for _array_element _actorcomponentlist
        (Default|SetSelectActor _array_element false)
        (Default|ShowTransformGizmo _array_element false)))
    (:NewEnumerator1
      (bind _actorcomponentlist_2 (CallFunction|GetEditorComponentActorList))
      (for _array_element_2 _actorcomponentlist_2
        (Default|SetSelectActor _array_element_2 false)))
    (:NewEnumerator2
      (bind _actorcomponentlist_3 (CallFunction|GetEditorComponentActorList))
      (for _array_element_3 _actorcomponentlist_3
        (Default|ShowTransformGizmo _array_element_3 false)))))

(fn AddModeChange
  (bind _dragmodelist (Variables|Default|GetDragModeList))
  (bind _dragmode (Variables|Default|GetDragMode))
  (bind _returnvalue (Utilities|Array|FindItem _dragmodelist _dragmode))
  (if (== (Utilities|Array|LastIndex _dragmodelist) _returnvalue)
    (ChangeMode|UpdateDragMode (Utilities|Array|Get(acopy) (Variables|Default|GetDragModeList)))
    (else
      (ChangeMode|UpdateDragMode (Utilities|Array|Get(acopy) (Variables|Default|GetDragModeList) (+ _returnvalue 1))))))

(fn UpdateHUDReleasePosition
  (if (Variables|Default|GetIsDrawButtonDown)
    (Default|UpdateReleasePosition (.AsBPC%20Drag%20Editor%20HUD (CallFunction|GetEditorComponentHUD)))))