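; Blueprint function library that looks up the transform gizmo's editor components on actors, the player controller and the HUD.
; Each lookup sends GetEditorComponentMessage to its target and casts the result to the matching drag-transform or multi-select component.
; The list function gathers drag-transform components from every actor implementing BPI_TransformComponent.
; The single lookups return a cast success flag, with controller and HUD taken from player index 0.
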(fn GetEditorComponentActorList
  (bind _outactors (Actor|GetAllActorswithInterface 0 "/TransformGizmoDepot/TransformGizmo/Blueprint/BPI_TransformComponent.BPI_TransformComponent_C"))
  (LocalVariables|SetTransformActorArray _outactors)
  (for _array_element (LocalVariables|GetTransformActorArray)
    (bind _component (Class|BPITransformComponent|GetEditorComponent(Message) _array_element))
    (bind _asbpc_drag_transform_actor (Utilities|Casting|CastToBPC_DragTransformActor _component))
    (Utilities|Array|Add (LocalVariables|GetActorComponentArray) _asbpc_drag_transform_actor))
  (return (LocalVariables|GetActorComponentArray)))

(fn GetEditorComponentController
  (bind _component (Class|BPITransformComponent|GetEditorComponent(Message) (Game|GetPlayerController 0)))
  (return (.AsBPC%20Drag%20Transform%20Controller (Utilities|Casting|CastToBPC_DragTransformController _component)) (.bSuccess (Utilities|Casting|CastToBPC_DragTransformController _component))))

(fn GetEditorComponentActor
  (params (目标 :type Object%20Object%20Reference))
  (bind _component (Class|BPITransformComponent|GetEditorComponent(Message) 目标))
  (return (.AsBPC%20Drag%20Transform%20Actor (Utilities|Casting|CastToBPC_DragTransformActor _component)) (.bSuccess (Utilities|Casting|CastToBPC_DragTransformActor _component))))

(fn GetEditorComponentHUD
  (bind _component (Class|BPITransformComponent|GetEditorComponent(Message) (HUD|GetHUD (Game|GetPlayerController 0))))
  (return (.AsBPC%20HUDMult%20Select (Utilities|Casting|CastToBPC_HUDMultSelect _component)) (.bSuccess (Utilities|Casting|CastToBPC_HUDMultSelect _component))))